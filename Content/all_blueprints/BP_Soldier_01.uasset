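; BP_Soldier_01 is a player soldier with axis-driven movement and unfinished mouse-based rotation.
; Forward/back and left/right inputs add movement along world X and Y.
; Tick calls UpdatePlayerRotation, which is empty apart from a disconnected GetMouseVelocity call.
; GetMouseVelocity divides mouse delta by frame time, while the unused dead-zone check compares a zero vector's length to MouseDeadZone rather than mouse velocity.
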(event EventTick
  (params (DeltaSeconds :type Float%20%28single-precision%29))
  (CallFunction|UpdatePlayerRotation))

(event Input|AxisEvents|InputAxisMoveForwardBack
  (params (AxisValue :type Float%20%28single-precision%29))
  (Pawn|Input|AddMovementInput (Math|Vector|MakeVector AxisValue 0.0 0.0) 1.0 false))

(event Input|AxisEvents|InputAxisMoveLeftRight
  (params (AxisValue :type Float%20%28single-precision%29))
  (Pawn|Input|AddMovementInput (Math|Vector|MakeVector 0.0 AxisValue 0.0) 1.0 false))

(fn ConstructionScript)

(fn UpdatePlayerRotation)

(fn GetMouseVelocity
  (bind _returnvalue (Game|GetPlayerController 0))
  (bind (_deltax _deltay) (Class|PlayerController|GetInputMouseDelta _returnvalue))
  (return (/ (Math|Vector2D|MakeVector2D _deltax _deltay) (Utilities|Time|GetWorldDeltaSeconds))))

(fn IsMouseDeadZone
  (return (> (Math|Vector2D|Vector2DLength) (Variables|Default|GetMouse%20Dead%20Zone))))